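; Base player Blueprint that exposes action state, life state and damage functions over its BPCPlayerProperty component.
; Action states form a unique-entry array with add, remove and find helpers, where find treats index 0 as absent; life state is a single value.
; Damage rewrites Health as Damage minus Health, floored at zero, keeping other stats, and the GetDamage event always passes zero.
; Tick, BeginPlay and the construction script are empty.
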(event EventBeginPlay)

(event Collision|EventActorBeginOverlap
  (params (OtherActor :type Actor%20Object%20Reference)))

(event EventTick
  (params (DeltaSeconds :type Float%20%28single-precision%29)))

(event EventGetDamage
  (params (BaseDamage :type Float%20%28single-precision%29))
  (CallFunction|FGetDamage 0.0))

(fn ConstructionScript)

(fn FGetPlayerActionState
  (return (Variables|/Game/Game/Player/Player/PlayerProperty/BPC_PlayerProperty.BPC_PlayerProperty_C|GetPlayerActionState (Variables|Default|GetBPC_PlayerProperty))))

(fn FSetPlayerActionState
  (params (NewPlayerAction :type E_PlayerActionState%20Enum :default "NewEnumerator0") (IsAdd :type Boolean))
  (bind _bpc_playerproperty (Variables|Default|GetBPC_PlayerProperty))
  (bind _playeractionstate (Variables|/Game/Game/Player/Player/PlayerProperty/BPC_PlayerProperty.BPC_PlayerProperty_C|GetPlayerActionState _bpc_playerproperty))
  (if IsAdd
    (Utilities|Array|AddUnique _playeractionstate NewPlayerAction)
    (else
      (Utilities|Array|RemoveItem _playeractionstate NewPlayerAction))))

(fn FFindPlayerActionState
  (params (ActionState :type E_PlayerActionState%20Enum :default "NewEnumerator0"))
  (return (> (Utilities|Array|FindItem (State|FGetPlayerActionState) ActionState) 0)))

(fn FGetPlayerLifeState
  (return (Variables|/Game/Game/Player/Player/PlayerProperty/BPC_PlayerProperty.BPC_PlayerProperty_C|GetPlayerLifeState (Variables|Default|GetBPC_PlayerProperty))))

(fn FSetPlayerLifeState
  (params (PlayerLifeState :type E_PlayerLifeState%20Enum :default "NewEnumerator0"))
  (Variables|/Game/Game/Player/Player/PlayerProperty/BPC_PlayerProperty.BPC_PlayerProperty_C|SetPlayerLifeState (Variables|Default|GetBPC_PlayerProperty) PlayerLifeState))

(fn FFindPlayerLifeState
  (params (LifeState :type E_PlayerLifeState%20Enum :default "NewEnumerator0"))
  (return (Utilities|Enum|Equal(Enum) (State|FGetPlayerLifeState) LifeState)))

(fn FGetDamage
  (params (Damage :type Float%20%28double-precision%29))
  (Variables|/Game/Game/Player/Player/PlayerProperty/BPC_PlayerProperty.BPC_PlayerProperty_C|SetCurrentProperty (Variables|Default|GetBPC_PlayerProperty) (Utilities|Struct|MakeF_CurrentPlayerProperty (Math|Float|SelectFloat 0.0 (- Damage (.Health (Utilities|Struct|BreakF_CurrentPlayerProperty (Variables|/Game/Game/Player/Player/PlayerProperty/BPC_PlayerProperty.BPC_PlayerProperty_C|GetCurrentProperty (Variables|Default|GetBPC_PlayerProperty))))) (< (- Damage (.Health (Utilities|Struct|BreakF_CurrentPlayerProperty (Variables|/Game/Game/Player/Player/PlayerProperty/BPC_PlayerProperty.BPC_PlayerProperty_C|GetCurrentProperty (Variables|Default|GetBPC_PlayerProperty))))) 0.0)) (.Shield (Utilities|Struct|BreakF_CurrentPlayerProperty (Variables|/Game/Game/Player/Player/PlayerProperty/BPC_PlayerProperty.BPC_PlayerProperty_C|GetCurrentProperty (Variables|Default|GetBPC_PlayerProperty)))) (.Stamina (Utilities|Struct|BreakF_CurrentPlayerProperty (Variables|/Game/Game/Player/Player/PlayerProperty/BPC_PlayerProperty.BPC_PlayerProperty_C|GetCurrentProperty (Variables|Default|GetBPC_PlayerProperty)))) (.Energy (Utilities|Struct|BreakF_CurrentPlayerProperty (Variables|/Game/Game/Player/Player/PlayerProperty/BPC_PlayerProperty.BPC_PlayerProperty_C|GetCurrentProperty (Variables|Default|GetBPC_PlayerProperty)))))))

(fn FGetPlayerBaseRef
  (return self))