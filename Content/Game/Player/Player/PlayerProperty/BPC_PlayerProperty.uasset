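; Player component that holds the player's base, real and current property sets (health, shield, stamina, energy) and manages stamina drain and regeneration.
; BeginPlay copies basic properties into real ones, applies walk speed to the player and fills current values to maximum.
; Mutually exclusive looping timers drain or delay-then-refill stamina with clamping, while one-off costs cancel regeneration.
; Tick restarts regeneration whenever stamina is below base maximum and neither timer runs.
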(event EventBeginPlay
  (Utilities|FlowControl|Sequence
    (:then_0
      (bind _player (Class|BPIGetPlayerClassInfo|FGetPlayerBaseRef(Message) (Components|GetOwner)))
      (Utilities|IsValid _player
        (:Is%20Valid
          (Variables|Default|SetPlayer _player))))
    (:then_1
      (bind _output_get (Variables|Default|SetRealProperty (Variables|Default|GetBasicProperty)))
      (Variables|/Script/Engine.CharacterMovementComponent|SetMaxWalkSpeed (Variables|/Script/Engine.Character|GetCharacterMovement (Variables|Default|GetPlayer)) (.MaxWalkSpeed (Utilities|Struct|BreakF_PlayerProperty _output_get)))
      (Utilities|Array|Add (Variables|Default|GetPlayerActionState) "NewEnumerator0"))
    (:then_2
      (Variables|Default|SetCurrentProperty (Utilities|Struct|MakeF_CurrentPlayerProperty (.MaxHealth (Utilities|Struct|BreakF_PlayerProperty (Variables|Default|GetRealProperty))) (.MaxShield (Utilities|Struct|BreakF_PlayerProperty (Variables|Default|GetRealProperty))) (.MaxStamina (Utilities|Struct|BreakF_PlayerProperty (Variables|Default|GetRealProperty))) (.MaxEnergy (Utilities|Struct|BreakF_PlayerProperty (Variables|Default|GetRealProperty))))))))

(event EventTick
  (params (DeltaSeconds :type Float%20%28single-precision%29))
  (Utilities|FlowControl|Sequence
    (:then_0
      (if (not (Utilities|Time|IsValidTimerHandle (Variables|Default|GetDecreaseStaminaTImer)))
        (if (not (Utilities|Time|IsValidTimerHandle (Variables|Default|GetIncreaseStaminaTimer)))
          (if (< (.Stamina (Utilities|Struct|BreakF_CurrentPlayerProperty (Variables|Default|GetCurrentProperty))) (.MaxStamina (Utilities|Struct|BreakF_PlayerProperty (Variables|Default|GetBasicProperty))))
            (Stamina|FSetIncreaseStaminaTimer)))))))

(fn FContinuetoDecreaseStamina
  (Variables|Default|SetCurrentProperty (Utilities|Struct|MakeF_CurrentPlayerProperty (.Health (Utilities|Struct|BreakF_CurrentPlayerProperty (Variables|Default|GetCurrentProperty))) (.Shield (Utilities|Struct|BreakF_CurrentPlayerProperty (Variables|Default|GetCurrentProperty))) (Math|Float|SelectFloat 0.0 (- (.Stamina (Utilities|Struct|BreakF_CurrentPlayerProperty (Variables|Default|GetCurrentProperty))) 8.0) (<= (- (.Stamina (Utilities|Struct|BreakF_CurrentPlayerProperty (Variables|Default|GetCurrentProperty))) 8.0) 0.0)) (.Energy (Utilities|Struct|BreakF_CurrentPlayerProperty (Variables|Default|GetCurrentProperty))))))

(fn FContinuetoIncreaseStamina
  (bind _realproperty (Variables|Default|GetRealProperty))
  (bind _maxstamina (Utilities|Struct|BreakF_PlayerProperty _realproperty))
  (Variables|Default|SetCurrentProperty (Utilities|Struct|MakeF_CurrentPlayerProperty (.Health (Utilities|Struct|BreakF_CurrentPlayerProperty (Variables|Default|GetCurrentProperty))) (.Shield (Utilities|Struct|BreakF_CurrentPlayerProperty (Variables|Default|GetCurrentProperty))) (Math|Float|SelectFloat _maxstamina (+ (.Stamina (Utilities|Struct|BreakF_CurrentPlayerProperty (Variables|Default|GetCurrentProperty))) 5.0) (>= (+ (.Stamina (Utilities|Struct|BreakF_CurrentPlayerProperty (Variables|Default|GetCurrentProperty))) 5.0) _maxstamina)) (.Energy (Utilities|Struct|BreakF_CurrentPlayerProperty (Variables|Default|GetCurrentProperty)))))
  (if (== (.MaxStamina (Utilities|Struct|BreakF_PlayerProperty (Variables|Default|GetRealProperty))) (.Stamina (Utilities|Struct|BreakF_CurrentPlayerProperty (Variables|Default|GetCurrentProperty))))
    (Utilities|Time|ClearandInvalidateTimerbyHandle (Variables|Default|GetIncreaseStaminaTimer))))

(fn FStaminaTimerControl
  (params (IsIncrease :type Boolean))
  (if IsIncrease
    (Stamina|FSetIncreaseStaminaTimer)
    (else
      (Stamina|FSetDecreaseStaminaTimer))))

(fn FSetIncreaseStaminaTimer
  (bind _decreasestaminatimer (Variables|Default|GetDecreaseStaminaTImer))
  (if (Utilities|Time|IsValidTimerHandle _decreasestaminatimer)
    (Utilities|Time|ClearandInvalidateTimerbyHandle _decreasestaminatimer))
  (if (not (Utilities|Time|IsValidTimerHandle (Variables|Default|GetIncreaseStaminaTimer)))
    (bind _returnvalue (Utilities|Time|SetTimerbyFunctionName 0 "F_ContinueToIncreaseStamina" 0.2 true 2.0))
    (Variables|Default|SetIncreaseStaminaTimer _returnvalue)))

(fn FSetDecreaseStaminaTimer
  (bind _increasestaminatimer (Variables|Default|GetIncreaseStaminaTimer))
  (if (Utilities|Time|IsValidTimerHandle _increasestaminatimer)
    (Utilities|Time|ClearandInvalidateTimerbyHandle _increasestaminatimer))
  (if (not (Utilities|Time|IsValidTimerHandle (Variables|Default|GetDecreaseStaminaTImer)))
    (bind _returnvalue (Utilities|Time|SetTimerbyFunctionName 0 "F_ContinueToDecreaseStamina" 0.2 true))
    (Variables|Default|SetDecreaseStaminaTImer _returnvalue)))

(fn FDecreaseStaminaOnce
  (params (DecreaseValue :type Float%20%28double-precision%29))
  (bind _increasestaminatimer (Variables|Default|GetIncreaseStaminaTimer))
  (if (Utilities|Time|IsValidTimerHandle _increasestaminatimer)
    (Utilities|Time|ClearandInvalidateTimerbyHandle _increasestaminatimer))
  (Variables|Default|SetCurrentProperty (Utilities|Struct|MakeF_CurrentPlayerProperty (.Health (Utilities|Struct|BreakF_CurrentPlayerProperty (Variables|Default|GetCurrentProperty))) (.Shield (Utilities|Struct|BreakF_CurrentPlayerProperty (Variables|Default|GetCurrentProperty))) (Math|Float|SelectFloat 0.0 (- (.Stamina (Utilities|Struct|BreakF_CurrentPlayerProperty (Variables|Default|GetCurrentProperty))) DecreaseValue) (<= (- (.Stamina (Utilities|Struct|BreakF_CurrentPlayerProperty (Variables|Default|GetCurrentProperty))) DecreaseValue) 0.0)) (.Energy (Utilities|Struct|BreakF_CurrentPlayerProperty (Variables|Default|GetCurrentProperty))))))