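; Player controller component for mouse-driven aiming and cursor-based camera offset of the controlled player.
; BeginPlay caches the controller, then after a short delay derives a pan range from camera FOV and height.
; Functions turn control yaw toward the cursor hit, draw a debug aim line, and shift the camera by mouse viewport position scaled to that range.
; Tick is empty, so these three functions rely on external callers.
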(event EventBeginPlay
  (Utilities|FlowControl|Sequence
    (:then_0
      (bind _controller (Class|BPIGetControllerClassInfo|FGetProjectXControllerRef(Message) (Components|GetOwner)))
      (Variables|Default|SetController _controller))
    (:then_1
      (Utilities|FlowControl|Delay 0.02)
      (CallFunction|FGetPlayerFOVRange))))

(event EventTick
  (params (DeltaSeconds :type Float%20%28single-precision%29)))

(fn FPlayerLookatMouse
  (bind _controller (Variables|Default|GetController))
  (bind (_hitresult _returnvalue) (Game|Player|GetHitResultUnderCursorbyChannel _controller "TraceTypeQuery1" true))
  (if _returnvalue
    (Pawn|SetControlRotation (Variables|Default|GetController) (Math|Rotator|MakeRotator 0.0 0.0 (.Yaw (Math|Rotator|BreakRotator (Math|Rotator|FindLookatRotation (Transformation|GetActorLocation (Variables|/Game/Game/Player/Controller/BP_ProjectXPlayerController.BP_ProjectXPlayerController_C|GetControlledPlayer (Variables|Default|GetController))) (.Location (Collision|BreakHitResult _hitresult)))))))))

(fn FDrawAimingDirection
  (bind _controller (Variables|Default|GetController))
  (bind _controlledplayer (Variables|/Game/Game/Player/Controller/BP_ProjectXPlayerController.BP_ProjectXPlayerController_C|GetControlledPlayer _controller))
  (bind _returnvalue (Transformation|GetActorLocation _controlledplayer))
  (Rendering|Debug|DrawDebugLine _returnvalue (+ _returnvalue (* (Math|Vector|GetForwardVector (Transformation|GetActorRotation _controlledplayer)) 1000)) "(R=1.000000,G=0.000000,B=0.295597,A=1.000000)" 0.0 0.0))

(fn FGetPlayerFOVRange
  (bind _controller (Variables|Default|GetController))
  (bind _controlledplayer (Variables|/Game/Game/Player/Controller/BP_ProjectXPlayerController.BP_ProjectXPlayerController_C|GetControlledPlayer _controller))
  (bind _camera (Variables|/Game/Game/Player/Player/BP_PlayerBase.BP_PlayerBase_C|GetCamera _controlledplayer))
  (Utilities|IsValid _controlledplayer
    (:Is%20Valid
      (bind _desiredview (Class|CameraComponent|GetCameraView _camera 0.0))
      (Variables|Default|SetFOVMaxRange (* (Math|Trig|Tan(Degrees) (/ (.FOV (Utilities|Struct|BreakMinimalViewInfo _desiredview)) 2.0)) (.Z (Math|Vector|BreakVector (Transformation|GetWorldLocation _camera))))))))

(fn FControlCameraPosition
  (bind _controller (Variables|Default|GetController))
  (bind _fovmaxrange (Variables|Default|GetFOVMaxRange))
  (bind _controller_2 (Variables|Default|GetController))
  (bind (_locationx _locationy _returnvalue) (Game|Player|GetMousePosition _controller_2))
  (bind (_sizex _sizey) (HUD|GetViewportSize _controller))
  (bind _returnvalue_2 (/ _locationy _sizey))
  (bind _returnvalue_3 (/ _locationx _sizex))
  (if _returnvalue
    (LocalVariables|SetMousePositionRate (Math|Vector2D|MakeVector2D _returnvalue_3 _returnvalue_2))
    (Utilities|FlowControl|Sequence
      (:then_0
        (LocalVariables|SetPlayerPositionRate (Math|Vector2D|MakeVector2D (- 1.0 (.X (Math|Vector2D|BreakVector2D (LocalVariables|GetMousePositionRate)))) (- 1.0 (.Y (Math|Vector2D|BreakVector2D (LocalVariables|GetMousePositionRate))))))
        (Utilities|FlowControl|Sequence
          (:then_0
            (LocalVariables|SetXSymbol (select (> (.X (Math|Vector2D|BreakVector2D (LocalVariables|GetPlayerPositionRate))) 0.5) -1.0 1.0)))
          (:then_1
            (LocalVariables|SetYSymbol (select (> (.Y (Math|Vector2D|BreakVector2D (LocalVariables|GetPlayerPositionRate))) 0.5) 1.0 -1.0)))
          (:then_2
            (LocalVariables|SetRealX (Math|Float|Absolute(Float) (- (.X (Math|Vector2D|BreakVector2D (LocalVariables|GetPlayerPositionRate))) 0.5)))
            (LocalVariables|SetRealY (Math|Float|Absolute(Float) (- (.Y (Math|Vector2D|BreakVector2D (LocalVariables|GetPlayerPositionRate))) 0.5))))
          (:then_3
            (LocalVariables|SetRealX (* (LocalVariables|GetRealX) (LocalVariables|GetXSymbol)))
            (LocalVariables|SetRealY (* (LocalVariables|GetYSymbol) (LocalVariables|GetRealY))))
          (:then_4
            (LocalVariables|SetCameraPositionOffset (Math|Vector2D|MakeVector2D (* (LocalVariables|GetRealX) _fovmaxrange) (* (LocalVariables|GetRealY) _fovmaxrange)))
            (Utilities|FlowControl|Sequence
              (:then_0
                (Transformation|SetRelativeLocation (Variables|/Game/Game/Player/Player/BP_PlayerBase.BP_PlayerBase_C|GetCamera (Variables|/Game/Game/Player/Controller/BP_ProjectXPlayerController.BP_ProjectXPlayerController_C|GetControlledPlayer (Variables|Default|GetController))) (Math|Vector|MakeVector 0.0 (.X (Math|Vector2D|BreakVector2D (LocalVariables|GetCameraPositionOffset))) (.Y (Math|Vector2D|BreakVector2D (LocalVariables|GetCameraPositionOffset)))) false false))
              (:then_1
                (if (Variables|Default|GetisDebug)
                  (Development|PrintString (Utilities|String|ToString(Float) (.X (Math|Vector2D|BreakVector2D (LocalVariables|GetCameraPositionOffset)))) true true "(R=0.000000,G=0.660000,B=1.000000,A=1.000000)" 0.0 "Move X : ")
                  (Development|PrintString (Utilities|String|ToString(Float) (.Y (Math|Vector2D|BreakVector2D (LocalVariables|GetCameraPositionOffset)))) true true "(R=0.000000,G=0.660000,B=1.000000,A=1.000000)" 0.0 "Move Y : ")))))
          (:then_5
            (if (Variables|Default|GetisDebug)
              (Development|PrintString (Utilities|String|Append "Real X : " (Utilities|String|ToString(Float) (LocalVariables|GetRealX))) true true "(R=0.000000,G=0.660000,B=1.000000,A=1.000000)" 0.0 "")
              (Development|PrintString (Utilities|String|Append "Real Y : " (Utilities|String|ToString(Float) (LocalVariables|GetRealY))) true true "(R=0.000000,G=0.660000,B=1.000000,A=1.000000)" 0.0 "")))
          (:then_6
            (if (Variables|Default|GetisDebug)
              (Development|PrintString (Utilities|String|Append "Player X : " (Utilities|String|ToString(Float) (- 1.0 (.X (Math|Vector2D|BreakVector2D (LocalVariables|GetMousePositionRate)))))) true true "(R=0.000000,G=0.660000,B=1.000000,A=1.000000)" 0.0 "")
              (Development|PrintString (Utilities|String|Append "Player Y : " (Utilities|String|ToString(Float) (- 1.0 (.Y (Math|Vector2D|BreakVector2D (LocalVariables|GetMousePositionRate)))))) true true "(R=0.000000,G=0.660000,B=1.000000,A=1.000000)" 0.0 "")))))
      (:then_1
        (if (Variables|Default|GetisDebug)
          (Development|PrintString (Utilities|String|Append "Mouse X : " (Utilities|String|ToString(Float) _returnvalue_3)) true true "(R=1.000000,G=0.091831,B=0.000000,A=1.000000)" 0.0 "")
          (Development|PrintString (Utilities|String|Append "Mouse Y : " (Utilities|String|ToString(Float) _returnvalue_2)) true true "(R=1.000000,G=0.058993,B=0.000000,A=1.000000)" 0.0 ""))))))