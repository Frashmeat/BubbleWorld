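; Player controller for ProjectX that turns Enhanced Input into movement, dive rolling, running, attack and aim on the controlled player.
; Movement follows fixed world axes, while an input control component drives mouse-facing (paused during rolls), camera position and debug aim drawing each tick.
; Actions add or remove entries in the player property component's action-state array.
; Rolling and running are gated by stamina, with rolls playing a montage toward velocity.
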(event Input|EnhancedActionEvents|EnhancedInputActionIA_MoveX
  (params (ActionValue :type Float%20%28double-precision%29) (ElapsedSeconds :type Float%20%28double-precision%29) (TriggeredSeconds :type Float%20%28double-precision%29) (InputAction :type Input%20Action%20Object%20Reference :default "/Game/Game/Player/Input/Action/IA_MoveX.IA_MoveX"))
  ;[1 0.4957 0.4259] Input
  ;;[1 1 1] Movement
  (Pawn|Input|AddMovementInput (Variables|Default|GetControlledPlayer) (Math|Vector|GetRightVector "0, 0, 0") ActionValue false))

(event Input|EnhancedActionEvents|EnhancedInputActionIA_MoveY
  (params (ActionValue :type Float%20%28double-precision%29) (ElapsedSeconds :type Float%20%28double-precision%29) (TriggeredSeconds :type Float%20%28double-precision%29) (InputAction :type Input%20Action%20Object%20Reference :default "/Game/Game/Player/Input/Action/IA_MoveY.IA_MoveY"))
  ;[1 0.4957 0.4259] Input
  ;;[1 1 1] Movement
  (Pawn|Input|AddMovementInput (Variables|Default|GetControlledPlayer) (Math|Vector|GetForwardVector "0, 0, 0") ActionValue false))

(event Input|EnhancedActionEvents|EnhancedInputActionIA_Aim
  (params (ActionValue :type Boolean) (ElapsedSeconds :type Float%20%28double-precision%29) (TriggeredSeconds :type Float%20%28double-precision%29) (InputAction :type Input%20Action%20Object%20Reference :default "/Game/Game/Player/Input/Action/IA_Aim.IA_Aim"))
  (bind _controlledplayer (Variables|Default|GetControlledPlayer))
  (bind _bpc_playerproperty (Variables|/Game/Game/Player/Player/BP_PlayerBase.BP_PlayerBase_C|GetBPC_PlayerProperty _controlledplayer))
  (bind _playeractionstate (Variables|/Game/Game/Player/Player/PlayerProperty/BPC_PlayerProperty.BPC_PlayerProperty_C|GetPlayerActionState _bpc_playerproperty))
  ;[1 1 1] Attack / Aim Control
  (:Triggered
    (Utilities|Array|AddUnique _playeractionstate "NewEnumerator1"))
  (:Completed
    (Utilities|Array|RemoveItem _playeractionstate "NewEnumerator1")))

(event Input|EnhancedActionEvents|EnhancedInputActionIA_HandheldWeaponAttack
  (params (ActionValue :type Boolean) (ElapsedSeconds :type Float%20%28double-precision%29) (TriggeredSeconds :type Float%20%28double-precision%29) (InputAction :type Input%20Action%20Object%20Reference :default "/Game/Game/Player/Input/Action/IA_HandheldWeaponAttack.IA_HandheldWeaponAttack"))
  (bind _controlledplayer (Variables|Default|GetControlledPlayer))
  (bind _bpc_playerproperty (Variables|/Game/Game/Player/Player/BP_PlayerBase.BP_PlayerBase_C|GetBPC_PlayerProperty _controlledplayer))
  (bind _playeractionstate (Variables|/Game/Game/Player/Player/PlayerProperty/BPC_PlayerProperty.BPC_PlayerProperty_C|GetPlayerActionState _bpc_playerproperty))
  ;[1 1 1] Attack / Aim Control
  (:Triggered
    (Utilities|Array|AddUnique _playeractionstate "NewEnumerator3"))
  (:Completed
    (Utilities|Array|RemoveItem _playeractionstate "NewEnumerator3")))

(event Input|EnhancedActionEvents|EnhancedInputActionIA_Run
  (params (ActionValue :type Boolean) (ElapsedSeconds :type Float%20%28double-precision%29) (TriggeredSeconds :type Float%20%28double-precision%29) (InputAction :type Input%20Action%20Object%20Reference :default "/Game/Game/Player/Input/Action/IA_Run.IA_Run"))
  (bind _controlledplayer (Variables|Default|GetControlledPlayer))
  (bind _controlledplayer_2 (Variables|Default|GetControlledPlayer))
  (bind _controlledplayer_3 (Variables|Default|GetControlledPlayer))
  (bind _charactermovement (Variables|/Script/Engine.Character|GetCharacterMovement _controlledplayer_2))
  (bind _bpc_playerproperty (Variables|/Game/Game/Player/Player/BP_PlayerBase.BP_PlayerBase_C|GetBPC_PlayerProperty _controlledplayer))
  (bind _bpc_playerproperty_2 (Variables|/Game/Game/Player/Player/BP_PlayerBase.BP_PlayerBase_C|GetBPC_PlayerProperty _controlledplayer_3))
  (bind _playeractionstate (Variables|/Game/Game/Player/Player/PlayerProperty/BPC_PlayerProperty.BPC_PlayerProperty_C|GetPlayerActionState _bpc_playerproperty_2))
  (bind _basicproperty (Variables|/Game/Game/Player/Player/PlayerProperty/BPC_PlayerProperty.BPC_PlayerProperty_C|GetBasicProperty _bpc_playerproperty_2))
  (bind (_maxhealth _maxshield _maxstamina _maxenergy _maxwalkspeed _maxrunspeed) (Utilities|Struct|BreakF_PlayerProperty _basicproperty))
  ;[1 0.4957 0.4259] Input
  (:Triggered
    (if (> (.Stamina (Utilities|Struct|BreakF_CurrentPlayerProperty (Variables|/Game/Game/Player/Player/PlayerProperty/BPC_PlayerProperty.BPC_PlayerProperty_C|GetCurrentProperty (Variables|/Game/Game/Player/Player/BP_PlayerBase.BP_PlayerBase_C|GetBPC_PlayerProperty (Variables|Default|GetControlledPlayer))))) 8.0)
      (Variables|/Script/Engine.CharacterMovementComponent|SetMaxWalkSpeed _charactermovement _maxrunspeed)
      (Utilities|Array|AddUnique _playeractionstate "NewEnumerator2")
      (Default|FStaminaTimerControl _bpc_playerproperty false)
      (else
        (Variables|/Script/Engine.CharacterMovementComponent|SetMaxWalkSpeed _charactermovement _maxwalkspeed :!label _label)
        (Utilities|Array|RemoveItem _playeractionstate "NewEnumerator2")
        (Default|FStaminaTimerControl _bpc_playerproperty true))))
  (:Completed
    (goto _label)))

(event Input|EnhancedActionEvents|EnhancedInputActionIA_Rolling
  (params (ActionValue :type Boolean) (ElapsedSeconds :type Float%20%28double-precision%29) (TriggeredSeconds :type Float%20%28double-precision%29) (InputAction :type Input%20Action%20Object%20Reference :default "/Game/Game/Player/Input/Action/IA_Rolling.IA_Rolling"))
  (bind _controlledplayer (Variables|Default|GetControlledPlayer))
  ;[1 0.4957 0.4259] Input
  (if (> (.Stamina (Utilities|Struct|BreakF_CurrentPlayerProperty (Variables|/Game/Game/Player/Player/PlayerProperty/BPC_PlayerProperty.BPC_PlayerProperty_C|GetCurrentProperty (Variables|/Game/Game/Player/Player/BP_PlayerBase.BP_PlayerBase_C|GetBPC_PlayerProperty (Variables|Default|GetControlledPlayer))))) 0.0)
    (if (not (>= (Utilities|Array|FindItem (Variables|/Game/Game/Player/Player/PlayerProperty/BPC_PlayerProperty.BPC_PlayerProperty_C|GetPlayerActionState (Variables|/Game/Game/Player/Player/BP_PlayerBase.BP_PlayerBase_C|GetBPC_PlayerProperty (Variables|Default|GetControlledPlayer))) "NewEnumerator4") 0))
      (Animation|Montage|PlayMontage (Variables|/Script/Engine.Character|GetMesh _controlledplayer) "/Game/Game/Player/Assist/Anim/Montage/A_DiveRoll_L_Vault_Retargeted_Montage.A_DiveRoll_L_Vault_Retargeted_Montage" 1.5
        (:then
          (Pawn|SetControlRotation (Math|Conversions|RotationFromXVector (Math|Vector|Normalize (Variables|/Script/Engine.MovementComponent|GetVelocity (Variables|/Script/Engine.Character|GetCharacterMovement _controlledplayer)))))
          (Utilities|Array|AddUnique (Variables|/Game/Game/Player/Player/PlayerProperty/BPC_PlayerProperty.BPC_PlayerProperty_C|GetPlayerActionState (Variables|/Game/Game/Player/Player/BP_PlayerBase.BP_PlayerBase_C|GetBPC_PlayerProperty (Variables|Default|GetControlledPlayer))) "NewEnumerator4")
          (Utilities|FlowControl|DoOnce false :!label _label
            (:Completed
              (Default|FDecreaseStaminaOnce (Variables|/Game/Game/Player/Player/BP_PlayerBase.BP_PlayerBase_C|GetBPC_PlayerProperty (Variables|Default|GetControlledPlayer)) 2e+01))))
        (:OnCompleted
          (Utilities|Array|RemoveItem (Variables|/Game/Game/Player/Player/PlayerProperty/BPC_PlayerProperty.BPC_PlayerProperty_C|GetPlayerActionState (Variables|/Game/Game/Player/Player/BP_PlayerBase.BP_PlayerBase_C|GetBPC_PlayerProperty (Variables|Default|GetControlledPlayer))) "NewEnumerator4")
          (goto _label Reset))))))

(event EventBeginPlay
  (Utilities|FlowControl|Sequence
    (:then_0
      ;[1 1 1] Init
      (|AddInputMapping))
    (:then_1
      (bind _player (Class|BPIGetPlayerClassInfo|FGetPlayerBaseRef(Message) (Pawn|GetControlledPawn)))
      (Variables|Default|SetControlledPlayer _player))))

(event EventTick
  (params (DeltaSeconds :type Float%20%28single-precision%29))
  (bind _controlledplayer (Variables|Default|GetControlledPlayer))
  (bind _bpc_playerinputcontrolcomponent (Variables|Default|GetBPC_PlayerInputControlComponent))
  (bind _bpc_playerproperty (Variables|/Game/Game/Player/Player/BP_PlayerBase.BP_PlayerBase_C|GetBPC_PlayerProperty _controlledplayer))
  (bind _playeractionstate (Variables|/Game/Game/Player/Player/PlayerProperty/BPC_PlayerProperty.BPC_PlayerProperty_C|GetPlayerActionState _bpc_playerproperty))
  (Utilities|FlowControl|Sequence
    (:then_0
      (if (not (>= (Utilities|Array|FindItem (Variables|/Game/Game/Player/Player/PlayerProperty/BPC_PlayerProperty.BPC_PlayerProperty_C|GetPlayerActionState (Variables|/Game/Game/Player/Player/BP_PlayerBase.BP_PlayerBase_C|GetBPC_PlayerProperty (Variables|Default|GetControlledPlayer))) "NewEnumerator4") 0))
        ;[1 1 1] Player Look / View Control
        (Default|FPlayerLookatMouse _bpc_playerinputcontrolcomponent)))
    (:then_1
      (Default|FControlCameraPosition _bpc_playerinputcontrolcomponent))
    (:then_2
      (if (Variables|Default|GetIsDebug)
        (Default|FDrawAimingDirection (Variables|Default|GetBPC_PlayerInputControlComponent))
        (Development|PrintString (Utilities|String|EnumtoString (Utilities|Array|Get(acopy) _playeractionstate (Utilities|Array|LastIndex _playeractionstate))) true true "(R=0.000000,G=0.660000,B=1.000000,A=1.000000)" 0.0)
        (Development|PrintString (Utilities|String|ToString(Float) (.Stamina (Utilities|Struct|BreakF_CurrentPlayerProperty (Variables|/Game/Game/Player/Player/PlayerProperty/BPC_PlayerProperty.BPC_PlayerProperty_C|GetCurrentProperty (Variables|/Game/Game/Player/Player/BP_PlayerBase.BP_PlayerBase_C|GetBPC_PlayerProperty (Variables|Default|GetControlledPlayer)))))) true true "(R=1.000000,G=0.905019,B=0.000000,A=1.000000)" 0.0)))))

(fn ConstructionScript)

(fn FCheckClass
  (return (== (Utilities|GetClass self) "BP_ProjectXPlayerController_C")))

(fn FGetProjectXControllerRef
  (return self))