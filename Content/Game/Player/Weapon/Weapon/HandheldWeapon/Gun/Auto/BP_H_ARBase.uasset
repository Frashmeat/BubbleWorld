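; Base Blueprint for automatic assault-rifle-style handheld guns, handling firing, ammo and reloading.
; Attack checks ammo and player action states, then a looping fire-rate timer spawns bullet actors until stopped or blocked.
; Random spread affects only yaw off control rotation; while aiming, it narrows as consecutive shots exceed the precision count.
; Reload sets a player action state, then a timer refills the magazine and clears it.
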(event EventBeginPlay
  (|CallParentFunction)
  (Variables|Default|SetCurrentBulletCount (.BulletCapacity (Utilities|Struct|BreakF_GunProperty (Variables|Default|GetRealGunProperty)))))

(event Collision|EventActorBeginOverlap
  (params (OtherActor :type Actor%20Object%20Reference))
  (|CallParentFunction OtherActor) ; 此节点被禁用，将不会被调用。\n从引脚连出引线来编译功能。
)

(event EventTick
  (params (DeltaSeconds :type Float%20%28single-precision%29))
  (|CallParentFunction DeltaSeconds))

(event EventFReload
  (Default|FSetPlayerActionState (Variables|Default|GetOwnedPlayer) "NewEnumerator5" true)
  (bind _returnvalue (Utilities|Time|SetTimerbyFunctionName 0 "F_Reloading" 2.0))
  (Variables|Default|SetBeginReloadTimer _returnvalue))

(event EventFAttack
  (bind _canattack (CallFunction|FCanAttack))
  (if _canattack
    (CallFunction|FBeginAttack)))

(event EventFStopAttack
  (bind _beginattacktimer (Variables|Default|GetBeginAttackTimer))
  (if (Utilities|Time|IsValidTimerHandle _beginattacktimer)
    (Utilities|Time|ClearandInvalidateTimerbyHandle _beginattacktimer)
    (Utilities|Array|RemoveItem (Default|FGetPlayerActionState (Variables|Default|GetOwnedPlayer)) "NewEnumerator3")
    (Variables|Default|SetContinuedShootCount 0)))

(fn ConstructionScript
  (|CallParentFunction))

(fn FCanAttack
  (bind _ownedplayer (Variables|Default|GetOwnedPlayer))
  (bind _bpc_playerproperty (Variables|/Game/Game/Player/Player/BP_PlayerBase.BP_PlayerBase_C|GetBPC_PlayerProperty _ownedplayer))
  (bind _playeractionstate (Variables|/Game/Game/Player/Player/PlayerProperty/BPC_PlayerProperty.BPC_PlayerProperty_C|GetPlayerActionState _bpc_playerproperty))
  (return (and (> (Variables|Default|GetCurrentBulletCount) 0) (Math|Boolean|ANDBoolean (== (Utilities|Array|FindItem _playeractionstate "NewEnumerator4") -1) (== (Utilities|Array|FindItem _playeractionstate "NewEnumerator5") -1) (== (Utilities|Array|FindItem _playeractionstate "NewEnumerator6") -1)))))

(fn FBeginAttack
  (Default|FSetPlayerActionState (Variables|Default|GetOwnedPlayer) "NewEnumerator3" true)
  (if (not (Utilities|Time|IsValidTimerHandle (Variables|Default|GetBeginAttackTimer)))
    (bind _returnvalue (Utilities|Time|SetTimerbyFunctionName 0 "F_Shoot" (/ 1.0 (/ (.ShootRate (Utilities|Struct|BreakF_GunProperty (Variables|Default|GetRealGunProperty))) 6e+01)) true))
    (Variables|Default|SetBeginAttackTimer _returnvalue)))

(fn FShoot
  (bind _canattack (CallFunction|FCanAttack))
  (if _canattack
    (CallFunction|FShootBullet (!= (Utilities|Array|FindItem (Variables|/Game/Game/Player/Player/PlayerProperty/BPC_PlayerProperty.BPC_PlayerProperty_C|GetPlayerActionState (Variables|/Game/Game/Player/Player/BP_PlayerBase.BP_PlayerBase_C|GetBPC_PlayerProperty (Variables|Default|GetOwnedPlayer))) "NewEnumerator1") -1))
    (else
      (CallFunction|FStopAttack))))

(fn FShootBullet
  (params (IsAiming :type Boolean))
  (for _index (range 0 (- (.ShootBulletCount (Utilities|Struct|BreakF_GunProperty (Variables|Default|GetRealGunProperty))) 1))
    (bind _direction (CallFunction|FCalculateShootDirection IsAiming))
    (Game|SpawnActorfromClass "/Game/Game/Player/Weapon/Bullet/BP_BulletBase.BP_BulletBase_C" (Math|Transform|MakeTransform (Transformation|GetActorLocation) _direction) "Undefined" "MultiplyWithRoot" 0 self 5e+03 0))
  (Math|Integer|DecrementInt (Variables|Default|GetCurrentBulletCount)
    (:%20%20
      (Math|Integer|IncrementInt (Variables|Default|GetContinuedShootCount)))))

(fn FCalculateShootDirection
  (params (IsAiming :type Boolean))
  (bind _realgunproperty (Variables|Default|GetRealGunProperty))
  (bind _continuedshootcount (Variables|Default|GetContinuedShootCount))
  (bind _precisioncount (Utilities|Struct|BreakF_GunProperty _realgunproperty))
  (bind _returnvalue (Math|Conversions|ToFloat(Integer) _continuedshootcount))
  (bind _returnvalue_2 (Math|Conversions|ToFloat(Integer) _precisioncount))
  (bind _returnvalue_3 (/ _returnvalue_2 _returnvalue))
  (bind _returnvalue_4 (> _returnvalue_3 1.0))
  (bind _returnvalue_5 (Math|Float|SelectFloat 1.0 _returnvalue_3 _returnvalue_4))
  (LocalVariables|SetBaseRotation (Pawn|GetControlRotation (Pawn|GetController (Variables|Default|GetOwnedPlayer)) :!class /Script/Engine.Controller))
  (if IsAiming
    (return (Math|Rotator|MakeRotator (.Roll (Math|Rotator|BreakRotator (LocalVariables|GetBaseRotation))) (.Pitch (Math|Rotator|BreakRotator (LocalVariables|GetBaseRotation))) (+ (.Yaw (Math|Rotator|BreakRotator (LocalVariables|GetBaseRotation))) (* (.ShootOffset (Utilities|Struct|BreakF_GunProperty (Variables|Default|GetRealGunProperty))) (Math|Random|RandomFloatinRange (* _returnvalue_5 -1.0) _returnvalue_5)))))
    (else
      (return (Math|Rotator|MakeRotator (.Roll (Math|Rotator|BreakRotator (LocalVariables|GetBaseRotation))) (.Pitch (Math|Rotator|BreakRotator (LocalVariables|GetBaseRotation))) (+ (.Yaw (Math|Rotator|BreakRotator (LocalVariables|GetBaseRotation))) (* (.ShootOffset (Utilities|Struct|BreakF_GunProperty (Variables|Default|GetRealGunProperty))) (Math|Random|RandomFloatinRange -1.0 1.0))))))))

(fn FReloading
  (Variables|Default|SetCurrentBulletCount (.BulletCapacity (Utilities|Struct|BreakF_GunProperty (Variables|Default|GetRealGunProperty))))
  (Default|FSetPlayerActionState (Variables|Default|GetOwnedPlayer) "NewEnumerator5" false))