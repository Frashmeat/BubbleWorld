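; Player weapon component that equips a handheld weapon and routes weapon input to it and to two shoulder weapon slots.
; On BeginPlay it caches the owning player, then spawns an AR weapon and snaps it to that player.
; Enhanced Input actions send message calls for attack, stop, reload and shoulder activation, leaving behavior to each weapon.
; Only the handheld slot is filled here; the shoulder weapons are not assigned in this graph.
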(event Input|EnhancedActionEvents|EnhancedInputActionIA_HandheldWeaponAttack
  (params (ActionValue :type Boolean) (ElapsedSeconds :type Float%20%28double-precision%29) (TriggeredSeconds :type Float%20%28double-precision%29) (InputAction :type Input%20Action%20Object%20Reference :default "/Game/Game/Player/Input/Action/IA_HandheldWeaponAttack.IA_HandheldWeaponAttack"))
  (bind _equipedhweapon (Variables|Default|GetEquipedHWeapon))
  (:Triggered
    (Class|BPIHandheldWeapon|FAttack(Message) _equipedhweapon))
  (:Completed
    (Class|BPIHandheldWeapon|FStopAttack(Message) _equipedhweapon)))

(event Input|EnhancedActionEvents|EnhancedInputActionIA_LeftShoulderWeapon
  (params (ActionValue :type Boolean) (ElapsedSeconds :type Float%20%28double-precision%29) (TriggeredSeconds :type Float%20%28double-precision%29) (InputAction :type Input%20Action%20Object%20Reference :default "/Game/Game/Player/Input/Action/IA_LeftShoulderWeapon.IA_LeftShoulderWeapon"))
  (Class|BPIShoulderCarryingWeapon|FActive(Message) (Variables|Default|GetLeftShoulderWeapon)))

(event Input|EnhancedActionEvents|EnhancedInputActionIA_Reload
  (params (ActionValue :type Boolean) (ElapsedSeconds :type Float%20%28double-precision%29) (TriggeredSeconds :type Float%20%28double-precision%29) (InputAction :type Input%20Action%20Object%20Reference :default "/Game/Game/Player/Input/Action/IA_Reload.IA_Reload"))
  (Class|BPIHandheldWeapon|FReload(Message) (Variables|Default|GetEquipedHWeapon)))

(event Input|EnhancedActionEvents|EnhancedInputActionIA_RighShoulderWeapon
  (params (ActionValue :type Boolean) (ElapsedSeconds :type Float%20%28double-precision%29) (TriggeredSeconds :type Float%20%28double-precision%29) (InputAction :type Input%20Action%20Object%20Reference :default "/Game/Game/Player/Input/Action/IA_RighShoulderWeapon.IA_RighShoulderWeapon"))
  (Class|BPIShoulderCarryingWeapon|FActive(Message) (Variables|Default|GetRightShoulderWeapon)))

(event EventBeginPlay
  (Utilities|FlowControl|Sequence
    (:then_0
      (bind _player (Class|BPIGetPlayerClassInfo|FGetPlayerBaseRef(Message) (Components|GetOwner)))
      (Variables|Default|SetOwner _player))
    (:then_1
      (bind _returnvalue (Game|SpawnActorfromClass :Class "/Game/Game/Player/Weapon/Weapon/HandheldWeapon/Gun/Auto/BP_H_ARBase.BP_H_ARBase_C" :SpawnTransform (Math|Transform|MakeTransform "0, 0, 0") :CollisionHandlingOverride "Undefined" :TransformScaleMethod "MultiplyWithRoot" :OwnedPlayer (Variables|Default|GetOwner) :Instigator 0))
      (bind _output_get (Variables|Default|SetEquipedHWeapon _returnvalue))
      (bind _returnvalue_2 (Transformation|AttachActorToActor _output_get (Variables|Default|GetOwner) "None" "SnapToTarget" "SnapToTarget" "SnapToTarget" true))
      (if _returnvalue_2
        _))))

(event EventTick
  (params (DeltaSeconds :type Float%20%28single-precision%29)))