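; AI controller for normal monsters that starts each monster's behavior tree and shuts it down when the monster is dying or dead.
; On BeginPlay it caches the player and controlled MonsterBase, then runs the tree found in DT_MonsterProperty under the monster's name.
; It binds to the monster's Dying and Dead delegates, stopping the brain component's logic if the life state is no longer Active.
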(event Custom|ControlBehaviorTree
  (bind _canrunbt (CallFunction|FCheckCanRunBehaviorTree))
  (if (not _canrunbt)
    (AI|Logic|StopLogic (Variables|Default|GetBrainComponent) "")))

(event EventBeginPlay
  (Utilities|FlowControl|Sequence
    (:then_0
      (bind _player (Class|BPIGetPlayerClassInfo|FGetPlayerBaseRef(Message) (Game|GetPlayerCharacter 0)))
      (Variables|Default|SetPlayer _player))
    (:then_1
      (bind _asmonster_base (Utilities|Casting|CastToMonsterBase (Pawn|GetControlledPawn)))
      (Variables|Default|SetControlledMonster _asmonster_base))
    (:then_2
      (bind _returnvalue (Utilities|GetDataTableRow "/Game/Game/Monster/DT_MonsterProperty.DT_MonsterProperty" (Variables|/Script/ProjectX.MonsterBase|GetMonsterName (Variables|Default|GetControlledMonster)))
        (:then
          (Variables|Default|SetBTAsset (.BTAsset (Utilities|Struct|BreakF_MonsterProperty _returnvalue)))
          (bind _btasset (Variables|Default|GetBTAsset)
            (:then
              (bind _returnvalue_2 (AI|RunBehaviorTree _btasset))
              (if (not _returnvalue_2)
                (Development|PrintString "Fail to Run Behavior Tree")))
            (:else
              (Development|PrintString "Behavior Asset is Null" :!label _label))))
        (:RowNotFound
          (goto _label))))
    (:then_3
      (EventDispatchers|BindEventtoMonsterDeadDelegate (Variables|Default|GetControlledMonster) (delegate Custom|ControlBehaviorTree))
      (EventDispatchers|BindEventtoMonsterDyingDelegate (Variables|Default|GetControlledMonster) (delegate Custom|ControlBehaviorTree)))))

(event EventTick
  (params (DeltaSeconds :type Float%20%28single-precision%29)))

(fn ConstructionScript)

(fn FCheckCanRunBehaviorTree
  (return (Utilities|Enum|Equal(Enum) (Variables|/Script/ProjectX.MonsterBase|GetMonsterLifeState (Variables|Default|GetControlledMonster)) "Active")))