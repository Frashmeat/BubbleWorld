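; Normal monster base Blueprint that loads monster stats and handles incoming damage.
; The construction script calls Init to copy base and attack properties from DT_MonsterProperty by MonsterName, printing an error on failure.
; TakeDamage affects only Active monsters, cutting damage sharply when piercing is below armor.
; A shield absorbs scaled hits without overflow into Health, and depleting either pool calls OnShieldBroken or OnDying.
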(event EventBeginPlay)

(event Collision|EventActorBeginOverlap
  (params (OtherActor :type Actor%20Object%20Reference)))

(event EventTick
  (params (DeltaSeconds :type Float%20%28single-precision%29)))

(fn ConstructionScript
  (bind _returnvalue (CallFunction|Init))
  (if (not _returnvalue)
    (Development|PrintString "Fail to Init")))

(fn TakeDamage
  (params (BaseDamage :type Float%20%28single-precision%29) (ShieldReduction :type Float%20%28single-precision%29) (ArmorPiercingLevel :type Integer))
  (if (Utilities|Enum|Equal(Enum) (Variables|Default|GetMonsterLifeState) "Active")
    (LocalVariables|SetRealDamage BaseDamage)
    (if (< ArmorPiercingLevel (Class|MonsterBase|GetArmor))
      (LocalVariables|SetRealDamage (* (LocalVariables|GetRealDamage) 0.1)))
    (if (> (Variables|Default|GetShield) 0.0)
      (LocalVariables|SetRealDamage (* (LocalVariables|GetRealDamage) ShieldReduction))
      (bind _output_get (Variables|Default|SetShield (Math|Float|SelectFloat 0.0 (- (Variables|Default|GetShield) (LocalVariables|GetRealDamage)) (< (- (Variables|Default|GetShield) (LocalVariables|GetRealDamage)) 0.0))))
      (if (<= _output_get 0.0)
        (Class|MonsterBase|OnShieldBroken))
      (return true)
      (else
        (bind _output_get_2 (Variables|Default|SetHealth (Math|Float|SelectFloat 0.0 (- (Variables|Default|GetHealth) (LocalVariables|GetRealDamage)) (< (- (Variables|Default|GetHealth) (LocalVariables|GetRealDamage)) 0.0))))
        (if (<= _output_get_2 0.0)
          (Class|MonsterBase|OnDying))
        (return true)))
    (else
      (return false))))

(fn Init
  (bind _returnvalue (Utilities|GetDataTableRow "/Game/Game/Monster/DT_MonsterProperty.DT_MonsterProperty" (Variables|Default|GetMonsterName))
    (:then
      (Utilities|FlowControl|Sequence
        (:then_0
          (Variables|Default|SetBasicMonsterBaseProperty (.MonsterBaseProperty (Utilities|Struct|BreakF_MonsterProperty _returnvalue))))
        (:then_1
          (Variables|Default|SetBasicMonsterAttackProperty (.MonsterAttackProperty (Utilities|Struct|BreakF_MonsterProperty _returnvalue)))
          (return true))))
    (:RowNotFound
      (return false))))