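; Crossbow spider monster that fires arrows at a victim when its Attack event runs, limited by a cooldown.
; Attack calls F_LaunchArrow when off cooldown, spawning an ArrowClass actor at the spider's location, rotated toward the victim's current position.
; Launching sets IsColding and starts a timer that calls F_Colding to clear it after ColdingTime.
; Each shot also draws a debug point at the victim.
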(event EventBeginPlay
  (|CallParentFunction))

(event Collision|EventActorBeginOverlap
  (params (OtherActor :type Actor%20Object%20Reference))
  (|CallParentFunction OtherActor) ; 此节点被禁用，将不会被调用。\n从引脚连出引线来编译功能。
)

(event EventTick
  (params (DeltaSeconds :type Float%20%28single-precision%29))
  (|CallParentFunction DeltaSeconds) ; 此节点被禁用，将不会被调用。\n从引脚连出引线来编译功能。
)

(event EventAttack
  (params (Victim :type Actor%20Object%20Reference))
  (Utilities|IsValid Victim
    (:Is%20Valid
      (if (not (Variables|Default|GetIsColding))
        (CallFunction|FLaunchArrow Victim)
        (Rendering|Debug|DrawDebugPoint (Transformation|GetActorLocation Victim) 1e+02 "(R=0.000000,G=0.122559,B=1.000000,A=1.000000)" 2.0)))))

(fn ConstructionScript
  (|CallParentFunction))

(fn FLaunchArrow
  (params (Victim :type Actor%20Object%20Reference))
  (bind _returnvalue (Transformation|GetActorLocation))
  (Utilities|IsValid Victim
    (:Is%20Valid
      (Game|SpawnActorfromClass (Variables|Default|GetArrowClass) (Math|Transform|MakeTransform _returnvalue (Math|Rotator|FindLookatRotation _returnvalue (Transformation|GetActorLocation Victim))) "Undefined" "MultiplyWithRoot" 0 0)
      (Utilities|FlowControl|Sequence
        (:then_0
          (Variables|Default|SetIsColding true))
        (:then_1
          (bind _returnvalue_2 (Utilities|Time|SetTimerbyFunctionName 0 "F_Colding" (Variables|Default|GetColdingTime)))
          (Variables|Default|SetColdingTimer _returnvalue_2))))))

(fn FColding
  (Variables|Default|SetIsColding false))